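; Gallery poster actor that appears only once all three inventory slots in the game instance hold items.
; On BeginPlay it reads the slot values from Game_Instance_Inv and sets the Cube's hidden state accordingly.
; Pressing E toggles a Poster_Information widget through a FlipFlop.
; Both begin and end overlap, as well as releasing E, enable input, so nothing here disables it.
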(event Collision|EventActorBeginOverlap
  (params (OtherActor :type Actor%20Object%20Reference))
  ;[1 1 1] Interaction with poster
  (Input|EnableInput (Game|GetPlayerController 0)))

(event EventBeginPlay
  ;[1 1 1] If inventory is over 1 then poster appears
  (bind _asgame_instance_inv (Utilities|Casting|CastToGame_Instance_Inv (Game|GetGameInstance))
    (:then
      (Development|SetHiddeninGame (Variables|Default|GetCube) (not (Math|Boolean|ANDBoolean (> (Variables|/Game/Inventory_Blueprints/Game_Instance_Inv.Game_Instance_Inv_C|GetInv_Slotitem_1 _asgame_instance_inv) 0) (> (Variables|/Game/Inventory_Blueprints/Game_Instance_Inv.Game_Instance_Inv_C|GetInv_Slotitem_2 _asgame_instance_inv) 0) (> (Variables|/Game/Inventory_Blueprints/Game_Instance_Inv.Game_Instance_Inv_C|GetInv_Slotitem_3 _asgame_instance_inv) 0))) false))
    (:CastFailed
      (Development|PrintString "item 1 - cast failed"))))

(event Collision|EventActorEndOverlap
  (params (OtherActor :type Actor%20Object%20Reference))
  ;[1 1 1] Interaction with poster
  (Input|EnableInput (Game|GetPlayerController 0)))

(event Input|KeyboardEvents|E
  (params (Key :type Key%20Structure :default "AnyKey"))
  ;[1 1 1] Interaction with poster
  (:Pressed
    (Utilities|FlowControl|FlipFlop
      (:A
        (bind _returnvalue (UserInterface|CreateWidget "/Game/Gallery/Blueprints/Widgets/Poster_Information.Poster_Information_C"))
        (UserInterface|Viewport|AddtoViewport _returnvalue 0))
      (:B
        (Widget|RemovefromParent _returnvalue))))
  (:Released
    (Input|EnableInput (Game|GetPlayerController 0))))

(fn ConstructionScript)