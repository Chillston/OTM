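; Spawn point actor for the Sanger Circus that keeps a Teddy present at its location.
; It spawns a Teddy on BeginPlay, then a looping one-second timer checks whether any Teddy still overlaps the actor.
; When none does, it schedules a replacement after a short random delay, with an IsRespawning flag preventing duplicate respawn timers.
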(event Custom|checkTeddy
  ;[1 1 1] Run every second to see if the teddy is gone
  (if (and (== (Utilities|Array|Length (Collision|GetOverlappingActors "/Game/Sanger_Circus/Teddy/blueprint/Teddy.Teddy_C" :!class /Script/Engine.Actor)) 0) (not (Variables|Default|GetIs%20Respawning)))
    (Variables|Default|SetIs%20Respawning true)
    (Utilities|Time|SetTimerbyEvent (delegate Custom|respawn) (Math|Random|RandomFloatinRange 1.0 3.0))))

(event Custom|respawn
  ;[1 1 1] Respawn
  (Game|SpawnActorfromClass "/Game/Sanger_Circus/Teddy/blueprint/Teddy.Teddy_C" (Math|Transform|MakeTransform (.Location (Math|Transform|BreakTransform (Transformation|GetActorTransform self))) "0,180.000000, 0") "Undefined" 0 0)
  (Variables|Default|SetIs%20Respawning false))

(event EventBeginPlay
  (Utilities|Time|SetTimerbyEvent (delegate Custom|checkTeddy) 1.0 true)
  (CallFunction|Respawn))

(fn ConstructionScript)